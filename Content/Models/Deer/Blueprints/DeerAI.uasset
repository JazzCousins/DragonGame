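; AI character Blueprint for a deer that wanders, pauses as if grazing, and flees when a DragonCharacter enters its sense volume.
; Tick switches between wandering toward random Target points and running away from the player until beyond range, always moving along the mesh's forward vector.
; Mesh yaw eases at speed-scaled rates, while a downward trace pitches it to the ground.
; Depleted health or E destroys it; tree-seeking food logic is unused.
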(event OnComponentBeginOverlap(Sences)
  (params (OtherActor :type Actor%20Object%20Reference) (OtherComp :type Primitive%20Component%20Object%20Reference) (OtherBodyIndex :type Integer) (bFromSweep :type Boolean) (SweepResult :type Hit%20Result%20Structure%20%28by%20ref%29))
  ;[1 1 1] Spot The dragon
  (bind _asdragon_character (Utilities|Casting|CastToDragonCharacter OtherActor))
  (Variables|Default|SetElerted true)
  (Variables|/Script/Engine.CharacterMovementComponent|SetMaxWalkSpeed (Variables|Character|GetCharacterMovement) (Variables|Default|GetMaxRunSpeed))
  (Variables|Default|SetLooking%20for%20food false))

(event Custom|wondering
  ;[1 1 1] Wondering
  (if (Variables|Default|GetLooking%20for%20food)
    ;[1 1 1] EatGrass
    (Utilities|FlowControl|DoOnce false :!label _label
      (:Completed
        (Variables|/Script/Engine.CharacterMovementComponent|SetMaxWalkSpeed (Variables|Character|GetCharacterMovement) 0.0)
        (Utilities|FlowControl|Delay (* (Variables|Default|Gettime) (Math|Random|RandomFloatinRange 0.1 1.0)))
        (Variables|Default|SetLooking%20for%20food false)
        (Variables|Default|Settime 0)
        (goto _label Reset)))
    (else
      (Utilities|FlowControl|Sequence
        (:then_0
          (Utilities|FlowControl|Delay (Math|Random|RandomFloatinRange 1.0 1e+01))
          (Variables|Default|SetLooking%20for%20food true))
        (:then_1
          (Variables|/Script/Engine.CharacterMovementComponent|SetMaxWalkSpeed (Variables|Character|GetCharacterMovement) (Variables|Default|GetMaxWalkingSpeed))
          (Transformation|SetWorldLocation (Variables|Default|GetTarget) (+ (Transformation|GetActorLocation) (Math|Vector|RotateVector (Math|Vector|MakeVector (Math|Random|RandomFloatinRange 0.0 1e+02) (Math|Random|RandomFloatinRange -1e+04 1e+04) 0.0) (Transformation|GetWorldRotation (Variables|Default|GetDeerMesh)))) false))))))

(event Custom|FindNewFood
  ;[1 0.03379 0] Not In Use
  ;;[1 1 1] check if deer is hungry
  (if (Variables|Default|GetLooking%20for%20food)
    ;;[1 1 1] FindNeerestFood
    (bind _outactors (Actor|GetAllActorsOfClass "/Game/Models/Plants/Trees/TreeBP.TreeBP_C"))
    (if (> (Utilities|Array|Length _outactors) 0)
      (for _array_element _outactors
        (if (> (Variables|Default|GetTreeDistance) (Math|Vector|VectorLength (- (Transformation|GetActorLocation _array_element) (Transformation|GetActorLocation))))
          (Variables|Default|SetTreeDistance (Math|Vector|VectorLength (- (Transformation|GetActorLocation _array_element) (Transformation|GetActorLocation))))
          (Transformation|SetWorldLocation (Variables|Default|GetTarget) (Transformation|GetActorLocation _array_element) false)))
      (Variables|Default|SetLooking%20for%20food false)
      (Variables|Default|SetEating true)
      (Variables|Default|SetTreeDistance 1e+06))))

(event Custom|RotateDeer
  (bind _returnvalue (Transformation|GetActorLocation))
  (bind _deermesh (Variables|Default|GetDeerMesh))
  (bind _deltatime (Variables|Default|GetDeltaTime))
  (bind _returnvalue_2 (Transformation|GetWorldRotation _deermesh))
  (bind (_pitch _yaw) (Class|KismetMathLibrary|BreakRot _returnvalue_2))
  ;[1 1 1] Rotates the deer
  (Transformation|SetWorldRotation _deermesh (Class|KismetMathLibrary|MakeRot (Math|Interpolation|FInterpTo _pitch (.Pitch (Class|KismetMathLibrary|BreakRot (Variables|Default|GetGroundAngle))) _deltatime 4.0) (Math|Interpolation|FInterpTo _yaw (.Yaw (Class|KismetMathLibrary|BreakRot (Math|Rotator|FindLookatRotation (Transformation|GetActorLocation) (Transformation|GetWorldLocation (Variables|Default|GetTarget))))) _deltatime (Math|Float|Clamp(Float) (/ (Variables|Default|GetWalkingSpeed) 8e+02) 0.01 5.0)) 0.0) false)
  (bind (_outhit _returnvalue_3) (Collision|LineTraceByChannel _returnvalue (- _returnvalue (Math|Vector|MakeVector 0.0 0.0 4e+04)) "TraceTypeQuery1" false 0 "None"))
  (if _returnvalue_3
    (Variables|Default|SetGroundAngle (Class|KismetMathLibrary|MakeRotfromYZ (Math|Vector|GetRightVector (Variables|Default|GetDeerMesh)) (.ImpactNormal (Collision|BreakHitResult _outhit))))))

(event Custom|Moves%20the%20deer
  ;[1 1 1] Movement
  (Variables|Default|SetWalkingSpeed (Math|Vector|VectorLength (Transformation|GetVelocity)))
  (Pawn|Input|AddMovementInput (Math|Vector|GetForwardVector (Variables|Default|GetDeerMesh)) 1.0 false)
  (Utilities|FlowControl|Delay 1.0)
  (Variables|Default|Settime (+ (Variables|Default|Gettime) 1)))

(event Custom|Run
  (bind _returnvalue (Transformation|GetActorLocation))
  (bind _deermesh (Variables|Default|GetDeerMesh))
  ;[1 1 1] RunAway
  (Transformation|SetWorldLocation (Variables|Default|GetTarget) (+ (Math|Vector|RotateVector (Math|Vector|MakeVector 4e+02 0.0 0.0) (Transformation|GetWorldRotation (Variables|Default|GetDeerMesh))) (Transformation|GetActorLocation)) false)
  (Transformation|SetWorldRotation _deermesh (Math|Interpolation|RInterpTo (Transformation|GetWorldRotation _deermesh) (Class|KismetMathLibrary|MakeRot (.Pitch (Class|KismetMathLibrary|BreakRot (Variables|Default|GetGroundAngle))) (.Yaw (Class|KismetMathLibrary|BreakRot (Math|Rotator|FindLookatRotation (Transformation|GetActorLocation (Game|GetPlayerCharacter 0)) (Transformation|GetActorLocation)))) 0.0) (Variables|Default|GetDeltaTime) (Math|Float|Clamp(Float) (/ (Variables|Default|GetWalkingSpeed) 8e+02) 0.001 1e+01)) false)
  (Utilities|FlowControl|Sequence
    (:then_0
      (if (> (Math|Vector|VectorLength (- (Transformation|GetActorLocation) (Transformation|GetActorLocation (Game|GetPlayerCharacter 0)))) 3e+03)
        (Variables|Default|SetElerted false)
        (Variables|/Script/Engine.CharacterMovementComponent|SetMaxWalkSpeed (Variables|Character|GetCharacterMovement) (Variables|Default|GetMaxWalkingSpeed))))
    (:then_1
      ;[1 1 1] Rotates the deer
      (bind (_outhit _returnvalue_2) (Collision|LineTraceByChannel _returnvalue (- _returnvalue (Math|Vector|MakeVector 0.0 0.0 4e+04)) "TraceTypeQuery1" false 0 "None"))
      (if _returnvalue_2
        (Variables|Default|SetGroundAngle (Class|KismetMathLibrary|MakeRotfromYZ (Math|Vector|GetRightVector (Variables|Default|GetDeerMesh)) (.ImpactNormal (Collision|BreakHitResult _outhit))))))))

(event EventAnyDamage
  (params (Damage :type Float%20%28single-precision%29) (DamageType :type Damage%20Type%20Object%20Reference) (InstigatedBy :type Controller%20Object%20Reference) (DamageCauser :type Actor%20Object%20Reference))
  (bind _deermesh (Variables|Default|GetDeerMesh))
  ;[1 1 1] TakeDamage
  (Variables|Default|SetHealth (- (Variables|Default|GetHealth) Damage))
  (if (<= (Variables|Default|GetHealth) 0.0)
    ;[1 1 1] Dead
    (Class|SkeletalMeshComponent|SetPhysicsBlendWeight _deermesh 1.0)
    (Physics|SetSimulatePhysics _deermesh true)
    (Class|SceneComponent|DetachfromParent true)
    (Actor|DestroyActor)))

(event EventTick
  (params (DeltaSeconds :type Float%20%28single-precision%29))
  ;[1 1 1] Updates Stuff!
  (Variables|Default|SetDeltaTime DeltaSeconds)
  (if (Variables|Default|GetElerted)
    (CallFunction|Run)
    (else
      (CallFunction|Wondering)
      (CallFunction|RotateDeer)))
  (CallFunction|MovestheDeer))

(event Input|KeyboardEvents|E
  (bind _deermesh (Variables|Default|GetDeerMesh))
  (:Pressed
    ;[1 1 1] Dead
    (Class|SkeletalMeshComponent|SetPhysicsBlendWeight _deermesh 1.0)
    (Physics|SetSimulatePhysics _deermesh true)
    (Class|SceneComponent|DetachfromParent true)
    (Actor|DestroyActor)))

(fn ConstructionScript)