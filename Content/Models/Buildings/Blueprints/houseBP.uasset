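; House building Blueprint with a Health value and a destructible component, set up to be broken by fire damage.
; Its disconnected fireDamage logic subtracts FireDamage hits from Health and, at zero or below, applies damage to the destructible with an impulse pointing away from the damage causer.
; The radial damage event is empty and that logic never runs, so the graph currently does nothing.
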(event EventRadialDamage
  (params (DamageReceived :type Float%20%28single-precision%29) (DamageType :type Damage%20Type%20Object%20Reference) (Origin :type Vector :default "0, 0, 0") (HitInfo :type Hit%20Result%20Structure%20%28by%20ref%29) (InstigatedBy :type Controller%20Object%20Reference) (DamageCauser :type Actor%20Object%20Reference)))

(fn ConstructionScript)