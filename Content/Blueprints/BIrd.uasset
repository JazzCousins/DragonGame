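; Player-controlled bird Blueprint with physics-driven flight, where movement input applies force and look input turns, pitches and banks the body.
; Pressing Jump flaps with an impulse and holds gliding, which damps sideways drift and reduces vertical velocity as forward speed rises.
; Tick also eases the camera toward the bird, widens FOV with speed and traces downward to set Landed.
; A delay-based flap cooldown exists but is disconnected.
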(event EventTick
  (params (DeltaSeconds :type Float%20%28single-precision%29))
  (bind _returnvalue (Transformation|GetVelocity))
  (bind _returnvalue_2 (Transformation|GetActorLocation))
  (bind _returnvalue_3 (Input|AxisValues|GetTurn))
  (bind _lookspeed (Variables|Default|GetLookSpeed))
  (bind _camera (Variables|Default|GetCamera))
  (bind _bird (Variables|Default|GetBird))
  (bind _camera_2 (Variables|Default|GetCamera))
  (bind _bird_2 (Variables|Default|GetBird))
  (bind _returnvalue_4 (Transformation|GetWorldRotation _bird))
  (bind _returnvalue_5 (Transformation|GetWorldRotation _bird_2))
  (bind _returnvalue_6 (Math|Vector|UnrotateVector _returnvalue _returnvalue_4))
  (bind (_pitch _yaw _roll) (Class|KismetMathLibrary|BreakRot _returnvalue_5))
  (bind (_x _y _z) (Math|Vector|BreakVector _returnvalue_6))
  (bind _returnvalue_7 (Math|Float|Clamp(Float) _x 0.0 8e+03))
  (Variables|Default|SetTime DeltaSeconds)
  (Physics|AddForce (Variables|Default|GetBird) (* (Math|Vector|RotateVector (Math|Vector|MakeVector (Input|AxisValues|GetMoveForward) (Input|AxisValues|GetMoveRight) 0.0) (Transformation|GetWorldRotation (Variables|Default|GetBird))) (Variables|Default|GetForwardforce)) "None")
  (if (Variables|Default|GetGliding)
    (Physics|SetPhysicsLinearVelocity (Variables|Default|GetBird) (Math|Vector|RotateVector (Math|Vector|MakeVector _returnvalue_7 (* _y 0.9) (/ _z (Math|Float|Clamp(Float) (/ _returnvalue_7 (Variables|Default|GetThurmalStrength)) 1.0 8e+03))) _returnvalue_4) false "None"))
  (Variables|/Script/Engine.CameraComponent|SetFieldOfView _camera_2 (Math|Interpolation|FInterpTo (Variables|/Script/Engine.CameraComponent|GetFieldOfView _camera_2) (+ (Math|Float|Clamp(Float) (/ _returnvalue_7 1e+02) 0.0 25.0) (Variables|Default|GetFOV)) (Variables|Default|GetTime) 2.0))
  (Transformation|SetWorldRotation (Variables|Default|GetCamera) (Math|Interpolation|RInterpTo (Transformation|GetWorldRotation _camera) (Math|Rotator|FindLookatRotation (Transformation|GetWorldLocation _camera) (Transformation|GetActorLocation)) (Variables|Default|GetTime) 4.0) false)
  (Transformation|SetWorldRotation (Variables|Default|GetBird) (Math|Interpolation|RInterpTo _returnvalue_5 (Class|KismetMathLibrary|MakeRot (Math|Float|ClampAngle (+ _pitch (* (Input|AxisValues|GetLookUp) (* _lookspeed -1.0))) -6e+01 8e+01) (+ _yaw (* _lookspeed _returnvalue_3)) (Math|Float|Clamp(Float) (Math|Interpolation|FInterpTo _roll (* _returnvalue_3 35.0) (Variables|Default|GetTime) 1.0) -35.0 35.0)) (Variables|Default|GetTime) 2e+01) false)
  (Variables|Default|SetLookY (Math|Interpolation|FInterpTo (Variables|Default|GetLookY) (* (Input|AxisValues|GetLookUp) -1.0) (Variables|Default|GetTime) 4.0))
  (Variables|Default|SetLookX (Math|Interpolation|FInterpTo (Variables|Default|GetLookX) (Input|AxisValues|GetTurn) (Variables|Default|GetTime) 4.0))
  (bind _returnvalue_8 (Collision|LineTraceByChannel _returnvalue_2 (- _returnvalue_2 "0, 0,100.000000") "TraceTypeQuery1" false 0 "None"))
  (if _returnvalue_8
    (Variables|Default|SetLanded true)
    (else
      (Variables|Default|SetLanded false))))

(event Input|ActionEvents|InputActionJump
  (bind _returnvalue (Input|AxisValues|GetMoveForward))
  (bind _returnvalue_2 (Input|AxisValues|GetMoveRight))
  (bind _bird (Variables|Default|GetBird))
  (bind _bird_2 (Variables|Default|GetBird))
  (bind _forwardforce (Variables|Default|GetForwardforce))
  (bind _returnvalue_3 (Transformation|GetWorldRotation _bird_2))
  (bind _returnvalue_4 (Math|Vector|MakeVector _returnvalue _returnvalue_2 0.0))
  (bind _returnvalue_5 (Transformation|GetWorldRotation _bird))
  (bind _returnvalue_6 (Math|Vector|RotateVector _returnvalue_4 _returnvalue_5))
  (bind _returnvalue_7 (* _returnvalue_6 _forwardforce))
  (bind _returnvalue_8 (Math|Vector|UnrotateVector _returnvalue_7 _returnvalue_3))
  (bind (_x _y) (Math|Vector|BreakVector _returnvalue_8))
  (:Pressed
    (Variables|Default|SetGliding true)
    (Physics|AddImpulse (Variables|Default|GetBird) (Math|Vector|RotateVector (Math|Vector|MakeVector _x (/ _y 4.0) 1e+03) _returnvalue_3) "None" false))
  (:Released
    (Variables|Default|SetGliding false)))

(fn ConstructionScript)