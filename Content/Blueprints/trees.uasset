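; Forest scatter actor that fills an area with randomly scaled oak and ash trees, which can be removed by damage or impact.
; The construction script uses a seeded stream and downward ground traces to place instanced meshes, favoring ash.
; Radial damage or fast-moving hits remove the hit index from Oak, falling back to Ash only if that fails.
; Destructible-mesh swapping and damage-driven bark heat logic are present but disconnected.
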(event EventHit
  (params (MyComp :type Primitive%20Component%20Object%20Reference) (Other :type Actor%20Object%20Reference) (OtherComp :type Primitive%20Component%20Object%20Reference) (bSelfMoved :type Boolean) (HitLocation :type Vector :default "0, 0, 0") (HitNormal :type Vector :default "0, 0, 0") (NormalImpulse :type Vector :default "0, 0, 0") (Hit :type Hit%20Result%20Structure%20%28by%20ref%29))
  (bind _hititem (Collision|BreakHitResult Hit))
  ;[1 1 1] DestroyOnCollision
  (if (> (Math|Vector|VectorLength (Transformation|GetVelocity Other)) 5e+02)
    (bind _returnvalue (Class|InstancedStaticMeshComponent|RemoveInstance (Variables|Default|GetOak) _hititem))
    (if (not _returnvalue)
      (Class|InstancedStaticMeshComponent|RemoveInstance (Variables|Default|GetAsh) _hititem))))

(event EventRadialDamage
  (params (DamageReceived :type Float%20%28single-precision%29) (DamageType :type Damage%20Type%20Object%20Reference) (Origin :type Vector :default "0, 0, 0") (HitInfo :type Hit%20Result%20Structure%20%28by%20ref%29) (InstigatedBy :type Controller%20Object%20Reference) (DamageCauser :type Actor%20Object%20Reference))
  (bind (_location _normal _impactpoint _impactnormal _physmat _hitactor _hitcomponent _hitbonename _hititem) (Collision|BreakHitResult HitInfo))
  ;[1 1 1] DestroyWhenDamaged
  (bind _returnvalue (Class|InstancedStaticMeshComponent|RemoveInstance (Variables|Default|GetOak) _hititem))
  (if (not _returnvalue)
    (Class|InstancedStaticMeshComponent|RemoveInstance (Variables|Default|GetAsh) _hititem)))

(fn ConstructionScript
  (bind _returnvalue (Transformation|GetActorLocation))
  (bind _randomstream (Variables|Default|GetRandomStream))
  (bind _treearearadius (Variables|Default|GetTreeAreaRadius))
  (bind _treearearadius_2 (Variables|Default|GetTreeAreaRadius))
  (bind _treenomber (Variables|Default|GetTreeNomber))
  (bind _randomstream_2 (Variables|Default|GetRandomStream))
  (bind _randomstream_3 (Variables|Default|GetRandomStream))
  (bind _returnvalue_2 (Math|Random|RandomFloatinRangefromStream 0.8 1.5 _randomstream_3))
  (bind _returnvalue_3 (* _treearearadius -1.0))
  (bind _returnvalue_4 (* _treearearadius_2 -1.0))
  (bind _returnvalue_5 (Math|Random|RandomFloatinRangefromStream _returnvalue_3 _treearearadius _randomstream))
  (bind _returnvalue_6 (Math|Random|RandomFloatinRangefromStream _returnvalue_4 _treearearadius_2 _randomstream_2))
  (bind _returnvalue_7 (Math|Vector|MakeVector _returnvalue_6 _returnvalue_5 0.0))
  (bind _returnvalue_8 (+ _returnvalue _returnvalue_7))
  (bind (_x _y) (Math|Vector|BreakVector _returnvalue_8))
  (bind _returnvalue_9 (Rendering|Material|CreateDynamicMaterialInstance "/Game/Matirials/Plants/OakBarkMat.OakBarkMat" :!class /Script/Engine.KismetMaterialLibrary))
  (Rendering|Material|SetMaterial (Variables|Default|GetOak) 0 _returnvalue_9)
  (Variables|Default|SetOakMaterial _returnvalue_9)
  ;[1 1 1] Getting Tree Locations
  (Utilities|Array|Clear _treenomber)
  (for _index (range 0 (Variables|Default|GetMaxNumberOfTrees))
    (bind _outhit (Collision|LineTraceForObjects _returnvalue_8 (Math|Vector|MakeVector _x _y -2e+03) (Variables|Default|GetGround) false 0 "None"))
    (Utilities|Array|Add _treenomber _index)
    ;[1 1 1] Creat oak or ash trees randomly
    (if (> (Math|Random|RandomIntegerinRangefromStream 1 4 (Variables|Default|GetRandomStream)) 1)
      (Class|InstancedStaticMeshComponent|AddInstanceWorldSpace (Variables|Default|GetAsh) (Math|Transform|MakeTransform (.Location (Collision|BreakHitResult _outhit)) "0, 0, 0" (Math|Vector|MakeVector _returnvalue_2 _returnvalue_2 _returnvalue_2)))
      (else
        (Class|InstancedStaticMeshComponent|AddInstanceWorldSpace (Variables|Default|GetOak) (Math|Transform|MakeTransform (.Location (Collision|BreakHitResult _outhit)) "0, 0, 0" (Math|Vector|MakeVector _returnvalue_2 _returnvalue_2 _returnvalue_2)))))))