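; DragonGameInstance is a game instance that handles hosting and joining multiplayer sessions.
; On init it runs a fullscreen console command.
; Hosting creates a non-LAN session sized by MaxPlayers and, on success, opens the multiplayer level as a listen server.
; Joining takes a search result passed into its event and joins that session, with both paths printing success or failure messages.
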(event Custom|JoinServerListEvent
  (params (NewParam :type Blueprint%20Session%20Result%20Structure))
  ;[1 1 1] JoinServer
  (|JoinSession (Game|GetPlayerController 0) NewParam
    (:OnSuccess
      (Development|PrintString "session joined" true true "(R=0.157399,G=1.000000,B=0.000000,A=1.000000)"))
    (:OnFailure
      (Development|PrintString "could not join session" true true "(R=1.000000,G=0.000000,B=0.055564,A=1.000000)"))))

(event Custom|HostGameEvent
  ;[1 1 1] hostGame
  (|Session (Game|GetPlayerController 0) (Variables|Default|GetMaxPlayers) false
    (:OnSuccess
      (Game|OpenLevel(byName) (Variables|Default|GetMultiplayerLevel) true "listen")
      (Development|PrintString "session created" true true "(R=0.084360,G=1.000000,B=0.000000,A=1.000000)"))
    (:OnFailure
      (Development|PrintString "could not create session" true true "(R=1.000000,G=0.000000,B=0.055564,A=1.000000)"))))

(event EventInit
  (Development|ExecuteConsoleCommand "FULLSCREEN" (Game|GetPlayerController 0)))