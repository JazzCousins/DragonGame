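; Sea monster NPC that chases the player's DragonCharacter every tick and turns to face it.
; It interpolates toward the player's X/Y at an inverted, offset height, so it moves opposite to the dragon vertically.
; Chase speed is recomputed from distance each frame, slowing as it closes in.
; A height check that would make it dive when the dragon climbs is present but disconnected.
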(event EventTick
  (params (DeltaSeconds :type Float%20%28single-precision%29))
  (Variables|Default|SetDeltaTime DeltaSeconds)
  (bind _asdragon_character (Utilities|Casting|CastToDragonCharacter (Game|Player|GetPlayerPawn 0)))
  ;[1 1 1] Chasing
  (Transformation|SetActorLocation (Math|Interpolation|VInterpTo (Transformation|GetActorLocation) (Math|Vector|MakeVector (.X (Math|Vector|BreakVector (Transformation|GetActorLocation _asdragon_character))) (.Y (Math|Vector|BreakVector (Transformation|GetActorLocation _asdragon_character))) (+ (* (.Z (Math|Vector|BreakVector (Transformation|GetActorLocation _asdragon_character))) -1.0) 1e+03)) (Variables|Default|GetDeltaTime) (Variables|Default|GetChaseSpeed)) false)
  ;[1 1 1] LooksAtThePlayer
  (Transformation|SetActorRotation (Math|Rotator|FindLookatRotation (Transformation|GetActorLocation) (Transformation|GetActorLocation _asdragon_character)))
  ;[1 1 1] SlowDownWhenGetClose
  (Variables|Default|SetChaseSpeed (/ (Math|Float|Clamp(Float) (- (Math|Vector|VectorLength (- (Transformation|GetActorLocation) (Transformation|GetActorLocation _asdragon_character))) 3.5e+03) 1.0 1e+04) 1.5e+04)))

(fn ConstructionScript)