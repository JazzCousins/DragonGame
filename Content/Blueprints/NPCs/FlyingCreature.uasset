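; Flying NPC creature that wanders toward an attraction point and chases the player's dragon when near, with a wider give-up radius.
; Tick eases rotation toward its target and sweeps it forward along its facing.
; While chasing, sharper angles to the player mean faster turning and slower flight; wandering is gentler, with slower animation.
; The construction script randomizes body and wing colors through a dynamic material; random-target logic is left disconnected.
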(event EventTick
  (params (DeltaSeconds :type Float%20%28single-precision%29))
  (bind _returnvalue (Transformation|GetActorRotation))
  (bind _returnvalue_2 (Transformation|GetActorLocation))
  (bind _returnvalue_3 (Transformation|GetActorLocation))
  (bind _returnvalue_4 (Transformation|GetActorRotation))
  (bind _returnvalue_5 (Math|Vector|UnrotateVector _returnvalue_2 _returnvalue))
  (bind _returnvalue_6 (Math|Vector|UnrotateVector _returnvalue_3 _returnvalue_4))
  (bind (_x _y _z) (Math|Vector|BreakVector _returnvalue_5))
  (bind (_x_2 _y_2 _z_2) (Math|Vector|BreakVector _returnvalue_6))
  (Variables|Default|SetDeltaTime DeltaSeconds)
  (Utilities|FlowControl|Sequence
    (:then_0
      (bind _asdragon_character (Utilities|Casting|CastToDragonCharacter (Game|Player|GetPlayerPawn 0)))
      (if (< (Math|Vector|VectorLength (- (Transformation|GetActorLocation _asdragon_character) (Transformation|GetActorLocation))) 3e+03)
        (Variables|Default|SetChasing true))
      (if (> (Math|Vector|VectorLength (- (Transformation|GetActorLocation _asdragon_character) (Transformation|GetActorLocation))) 1e+04)
        (Variables|Default|SetChasing false)))
    (:then_1
      (if (Variables|Default|GetChasing)
        ;[1 1 1] chasing movement
        (bind _asdragon_character_2 (Utilities|Casting|CastToDragonCharacter (Game|Player|GetPlayerPawn 0)))
        (Transformation|SetActorRotation (Math|Interpolation|RInterpTo _returnvalue_4 (Math|Rotator|FindLookatRotation (Transformation|GetActorLocation) (Transformation|GetActorLocation _asdragon_character_2)) (Variables|Default|GetDeltaTime) (Math|Float|Lerp 0.5 0.8 (/ (Class|KismetMathLibrary|DegAcos (Math|Vector|DotProduct (Math|Vector|GetForwardVector (Math|Rotator|FindLookatRotation (Transformation|GetActorLocation) (Transformation|GetActorLocation _asdragon_character_2))) (Math|Vector|GetForwardVector (Transformation|GetActorRotation)))) 1.8e+02))))
        (Transformation|SetActorLocation (Math|Interpolation|VInterpTo _returnvalue_3 (Math|Vector|RotateVector (Math|Vector|MakeVector (+ _x_2 2e+02) _y_2 _z_2) _returnvalue_4) (Variables|Default|GetDeltaTime) (Math|Float|Lerp 15.0 3.0 (/ (Class|KismetMathLibrary|DegAcos (Math|Vector|DotProduct (Math|Vector|GetForwardVector (Math|Rotator|FindLookatRotation (Transformation|GetActorLocation) (Transformation|GetActorLocation _asdragon_character_2))) (Math|Vector|GetForwardVector (Transformation|GetActorRotation)))) 1.8e+02))) true)
        (Components|Timeline|SetPlayRate (Variables|Default|GetSkeletalMesh1) 1.0)
        (else
          ;[1 1 1] rambling movement
          (Transformation|SetActorRotation (Math|Interpolation|RInterpTo _returnvalue (Math|Rotator|FindLookatRotation (Transformation|GetActorLocation) (Variables|Default|GetAttractionLocation)) (Variables|Default|GetDeltaTime) 0.2))
          (Transformation|SetActorLocation (Math|Interpolation|VInterpTo _returnvalue_2 (Math|Vector|RotateVector (Math|Vector|MakeVector (+ _x 2e+02) _y _z) _returnvalue) (Variables|Default|GetDeltaTime) 8.0) true)
          (Components|Timeline|SetPlayRate (Variables|Default|GetSkeletalMesh1) 0.5))))))

(fn ConstructionScript
  (bind _returnvalue (Rendering|Material|CreateDynamicMaterialInstance (Variables|Default|GetSkeletalMesh1) 0 "/Game/Dragon/TextureMaps/OtherDragon.OtherDragon" :!class /Script/Engine.PrimitiveComponent))
  (Rendering|Material|SetScalarParameterValue _returnvalue "Colour" (Math|Random|RandomFloatinRange 0.0 1.0) :!class /Script/Engine.MaterialInstanceDynamic)
  (Rendering|Material|SetVectorParameterValue _returnvalue "WingColour" (Utilities|Struct|MakeLinearColor (Math|Random|RandomFloatinRange 0.0 1.0) (Math|Random|RandomFloatinRange 0.0 1.0) (Math|Random|RandomFloatinRange 0.0 1.0) 1.0) :!class /Script/Engine.MaterialInstanceDynamic))